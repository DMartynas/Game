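; BP_SplineCreator is a railway helper actor that labels the points of its SplineDrawingCopier spline with their index numbers.
; The construction script stores the current spline length, then adds a text render component at each point, raised above it and matching its rotation.
; The event graph holds no active logic, so all work happens at construction time.
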(event EventBeginPlay)

(event Collision|EventActorBeginOverlap
  (params (OtherActor :type Actor%20Object%20Reference)))

(event EventTick
  (params (DeltaSeconds :type Float%20%28single-precision%29)))

(fn ConstructionScript
  (bind _spline_drawing_copier (Variables|Default|GetSpline_Drawing_Copier))
  ;[1 1 1] Add a text render to every point of the spline created
  (Variables|Default|SetCurrentSplineLength (Spline|GetSplineLength (Variables|Default|GetSpline_Drawing_Copier)))
  (for _index (range 0 (- (Spline|GetNumberOfSplinePoints (Variables|Default|GetSpline_Drawing_Copier)) 1))
    (bind _returnvalue (AddComponent|AddTextRenderComponent false))
    (Transformation|SetWorldTransform _returnvalue (Math|Transform|MakeTransform (+ (Spline|GetLocationatSplinePoint _spline_drawing_copier _index "World") "0, 0,100.000000") (Spline|GetRotationatSplinePoint _spline_drawing_copier _index "World")) false true)
    (Rendering|Components|TextRender|SetText _returnvalue (Utilities|Text|ToText(String) (Utilities|String|ToString(Integer) _index)))))