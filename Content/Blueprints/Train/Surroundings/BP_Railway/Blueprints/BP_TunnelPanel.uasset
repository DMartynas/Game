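; BP_TunnelPanel is a railway tunnel sign actor that displays a tunnel's name and its length in meters.
; On BeginPlay it fills the W_TunnelPanel widget on PanelF, converting the length to whole meters.
; A looping one-second timer then hides the actor beyond PanelCullDistance from the player camera and shows it within range.
; Despite the IsOnViewPort name, culling is purely distance-based, and the panel stays visible without a valid camera manager.
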(event Custom|IsOnViewPort?
  (bind _returnvalue (Game|GetPlayerCameraManager 0))
  ;[1 1 1] Hide actor when not on viewport
  (Utilities|IsValid _returnvalue
    (:Is%20Valid
      (if (< (Math|Vector|VectorLength (- (Transformation|GetActorLocation _returnvalue) (Transformation|GetActorLocation self))) (Variables|Default|GetPanelCullDistance))
        (if (Variables|Default|GetHidden) :!label _label
          (Rendering|SetActorHiddenInGame false)
          (Variables|Default|SetHidden false))
        (elif (not (Variables|Default|GetHidden))
          (Rendering|SetActorHiddenInGame true)
          (Variables|Default|SetHidden true))))
    (:Is%20Not%20Valid
      (goto _label))))

(event EventBeginPlay
  ;[0.07789 1 0.1636] Setup Panel Infos
  (bind _asw_tunnel_panel (Utilities|Casting|CastToW_TunnelPanel (UserInterface|GetUserWidgetObject (Variables|Default|GetPanel_F))))
  (Variables|/Game/UI/TrainTemplate/W_TunnelPanel.W_TunnelPanel_C|SetTunnelName _asw_tunnel_panel (Variables|Default|GetTunnelName_P))
  (Variables|/Game/UI/TrainTemplate/W_TunnelPanel.W_TunnelPanel_C|SetTunnelLength _asw_tunnel_panel (Utilities|Text|ToText(String) (Utilities|String|Append (Utilities|String|ToString(Integer) (Math|Float|Floor (/ (Variables|Default|GetTunnelLength_P) 1e+02))) " m")))
  (Utilities|Time|SetTimerbyEvent (delegate Custom|IsOnViewPort?) 1.0 true))

(fn ConstructionScript)