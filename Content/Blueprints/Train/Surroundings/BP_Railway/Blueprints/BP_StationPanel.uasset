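; Railway station panel actor that logs passing trains and hosts a 3D station clock widget, which receives a reference to the panel.
; A looping timer sphere-traces across the tracks for non-derailed carriages and resolves each to its convoy through the train spawner's list.
; New sightings are recorded with time, track and stop status, using a roughly five-minute duplicate check by train name.
; Another timer hides the panel beyond a camera cull distance.
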(event Custom|IsOnViewPort?
  (bind _returnvalue (Game|GetPlayerCameraManager 0))
  ;[1 1 1] On a delay we check if the panel is on screen, if it is not then set hidden in game
  (Utilities|IsValid _returnvalue
    (:Is%20Valid
      (if (< (Math|Vector|VectorLength (- (Transformation|GetActorLocation _returnvalue) (Transformation|GetActorLocation self))) (Variables|Default|GetPanelCullDistance))
        (if (Variables|Default|GetHidden) :!label _label
          (Variables|Default|SetHidden false))
        (elif (not (Variables|Default|GetHidden))
          (Variables|Default|SetHidden true))))
    (:Is%20Not%20Valid
      (goto _label))))

(event Custom|CheckTrains
  (bind _returnvalue (Transformation|GetActorLocation))
  (bind _returnvalue_2 (Math|DateTime|Now))
  (bind _railway_ref (Variables|Default|GetRailway_REf))
  (bind (_outhits _returnvalue_3) (Collision|MultiSphereTraceForObjects _returnvalue (+ _returnvalue (* (Math|Vector|GetForwardVector (Transformation|GetWorldRotation (Variables|Default|GetStaticMesh))) (* (Variables|/Game/Blueprints/Train/Surroundings/BP_RailWay/Blueprints/BP_RailWay.BP_RailWay_C|GetNumberOfTracks _railway_ref) (Variables|/Game/Blueprints/Train/Surroundings/BP_RailWay/Blueprints/BP_RailWay.BP_RailWay_C|GetTrackSeparation _railway_ref)))) 2e+02 (Utilities|Array|MakeArray "ObjectTypeQuery9") false 0 (Variables|Default|GetDebugTrainSearchTrace)))
  (if _returnvalue_3
    (for _array_element _outhits
      (bind _asbp_carriage_master (Utilities|Casting|CastToBP_Carriage_Master (.HitActor (Collision|BreakHitResult _array_element))))
      (if (not (Variables|/Game/Blueprints/Train/Carriage/BP_Carriage_Master/Blueprints/BP_Carriage_Master.BP_Carriage_Master_C|GetCarriageIsDerailed _asbp_carriage_master))
        (bind (_lv_foundresult1 _array_element_2) (CallFunction|FGetConvoyST _asbp_carriage_master))
        (if _lv_foundresult1
          (bind _lv_add1 (CallFunction|FCheckifAlreadyRecorded _array_element_2))
          (if _lv_add1
            (Variables|Default|SetCurrentTrainAtStation _array_element_2)
            (Utilities|Array|Add (Variables|Default|GetPassedTrains_0) (Utilities|Struct|MakeST_StationPanelRecord (Variables|Default|GetCurrentTrainAtStation) (.hour _returnvalue_2) (.minute _returnvalue_2) (Math|Integer|SelectInt 0 (Math|Integer|SelectInt 1 2 (Variables|/Game/Blueprints/Train/Carriage/BP_Carriage_Master/Blueprints/BP_Carriage_Master.BP_Carriage_Master_C|GetShouldStopAtStation? _asbp_carriage_master)) (Variables|/Game/Blueprints/Train/Carriage/BP_Carriage_Master/Blueprints/BP_Carriage_Master.BP_Carriage_Master_C|GetIsStoppingAtStation _asbp_carriage_master)) (Variables|/Game/Blueprints/Train/Carriage/BP_Bogie/Blueprints/BP_Bogie.BP_Bogie_C|GetBogie_Rail_ID (Variables|/Game/Blueprints/Train/Carriage/BP_Carriage_Master/Blueprints/BP_Carriage_Master.BP_Carriage_Master_C|GetBogie_F_REF _asbp_carriage_master))))))))))

(event Custom|CreateReferences
  ;[0.07789 1 0.1636] Setup Panel Infos
  (bind _asw_station_clock_3d_w (Utilities|Casting|CastToW_StationClock_3dW (UserInterface|GetUserWidgetObject (Variables|Default|GetPanel_F))))
  (Variables|/Game/UI/TrainTemplate/W_StationClock_3dW.W_StationClock_3dW_C|SetPanel_REF _asw_station_clock_3d_w self))

(event EventBeginPlay
  (Utilities|FlowControl|Delay 1.0)
  (bind _outactors (Actor|GetAllActorsOfClass 0))
  (if (> (Utilities|Array|Length _outactors) 0)
    ;[0.07789 1 0.1636] Setup Panel Infos
    (Variables|Default|SetTrainSpawner_REF 0))
  (CallFunction|CreateReferences)
  ;[1 1 1] Train checker timer
  (Utilities|Time|SetTimerbyEvent (delegate Custom|CheckTrains) (Variables|Default|GetCheck%20for%20trains%20each) true)
  ;[1 1 1] On a delay we check if the panel is on screen, if it is not then set hidden in game
  (Utilities|Time|SetTimerbyEvent (delegate Custom|IsOnViewPort?) 3.0 true))

(fn ConstructionScript)

(fn FGetConvoyST
  (params (CarriageFound :type BP%20Carriage%20Master%20Object%20Reference))
  (Utilities|IsValid (Variables|Default|GetTrainSpawner_REF)
    (:Is%20Valid
      (bind _array_element (Utilities|Array|ForEachLoopwithBreak (Variables|/Game/Blueprints/Train/Surroundings/BP_TrainSpawner/Blueprints/BP_Train_Spawner.BP_Train_Spawner_C|GetTrainsToSpawn (Variables|Default|GetTrainSpawner_REF)) :!label _label)
        (:LoopBody
          (bind _array_element_2 (Utilities|Array|ForEachLoopwithBreak (.AssignedCarriagesReadOnly (Utilities|Struct|BreakST_Convoy _array_element)) :!label _label_2)
            (:LoopBody
              (Utilities|IsValid _array_element_2
                (:Is%20Valid
                  (if (== _array_element_2 CarriageFound)
                    (LocalVariables|SetLV_Found_ST _array_element)
                    (LocalVariables|SetLV_FoundResult true)
                    (Utilities|FlowControl|Sequence
                      (:then_0
                        (goto _label_2 Break))
                      (:then_1
                        (goto _label Break)))))))))
        (:Completed
          (return (LocalVariables|GetLV_FoundResult) (LocalVariables|GetLV_Found_ST)))))
    (:Is%20Not%20Valid
      (return (LocalVariables|GetLV_FoundResult) (LocalVariables|GetLV_Found_ST)))))

(fn FCheckifAlreadyRecorded
  (params (InputPin :type ST%20Convoy%20Structure%20%28by%20ref%29))
  (bind _returnvalue (Math|DateTime|Now))
  (LocalVariables|SetLV_Add true)
  (bind _array_element (Utilities|Array|ForEachLoopwithBreak (Variables|Default|GetPassedTrains_0) :!label _label)
    (:LoopBody
      (if (Utilities|Enum|Equal(Enum) (.TrainName (Utilities|Struct|BreakST_Convoy (.Train (Utilities|Struct|BreakST_StationPanelRecord _array_element)))) (.TrainName (Utilities|Struct|BreakST_Convoy InputPin)))
        (if (or (and (== (.hour _returnvalue) (.Hours (Utilities|Struct|BreakST_StationPanelRecord _array_element))) (< (.minute _returnvalue) (+ (.Minutes (Utilities|Struct|BreakST_StationPanelRecord _array_element)) 5))) (and (== (.hour _returnvalue) (+ (.Hours (Utilities|Struct|BreakST_StationPanelRecord _array_element)) 1)) (< (.Minutes (Utilities|Struct|BreakST_StationPanelRecord _array_element)) 5)))
          (LocalVariables|SetLV_Add false)
          (goto _label Break))))
    (:Completed
      (return (LocalVariables|GetLV_Add)))))