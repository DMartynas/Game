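; BP_StationNamePanel is a railway station sign actor that displays the station name and track number on two widget components.
; On BeginPlay it copies both values into each W_StationNamePanel widget, then starts a looping timer.
; The timer hides the actor beyond a cull distance from the player camera manager and shows it again when near, tracking state to avoid redundant calls.
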(event Custom|IsOnViewPort?
  (bind _returnvalue (Game|GetPlayerCameraManager 0))
  ;[1 1 1] On a 3 seconds delay we check if the panel is nearby player. If it is not then set hidden in game
  (Utilities|IsValid (Game|GetPlayerController 0)
    (:Is%20Valid
      (Utilities|IsValid _returnvalue
        (:Is%20Valid
          (if (< (Math|Vector|VectorLength (- (Transformation|GetActorLocation _returnvalue) (Transformation|GetActorLocation self))) (Variables|Default|GetPanelCullDistance))
            (if (Variables|Default|GetHidden) :!label _label
              (Rendering|SetActorHiddenInGame false)
              (Variables|Default|SetHidden false))
            (elif (not (Variables|Default|GetHidden))
              (Rendering|SetActorHiddenInGame true)
              (Variables|Default|SetHidden true))))
        (:Is%20Not%20Valid
          (goto _label))))))

(event EventBeginPlay
  ;[1 1 1] Create widget references and set the station name panel
  (bind _asw_station_name_panel (Utilities|Casting|CastToW_StationNamePanel (UserInterface|GetUserWidgetObject (Variables|Default|GetWidget1))))
  (Variables|/Game/UI/TrainTemplate/W_StationNamePanel.W_StationNamePanel_C|SetStation%20Name _asw_station_name_panel (Variables|Default|GetStationName_P))
  (Variables|/Game/UI/TrainTemplate/W_StationNamePanel.W_StationNamePanel_C|SetTrack_index _asw_station_name_panel (Variables|Default|GetTrackN))
  (bind _asw_station_name_panel_2 (Utilities|Casting|CastToW_StationNamePanel (UserInterface|GetUserWidgetObject (Variables|Default|GetWidget))))
  (Variables|/Game/UI/TrainTemplate/W_StationNamePanel.W_StationNamePanel_C|SetStation%20Name _asw_station_name_panel_2 (Variables|Default|GetStationName_P))
  (Variables|/Game/UI/TrainTemplate/W_StationNamePanel.W_StationNamePanel_C|SetTrack_index _asw_station_name_panel_2 (Variables|Default|GetTrackN))
  (Utilities|Time|SetTimerbyEvent (delegate Custom|IsOnViewPort?) 3.0 true))

(fn ConstructionScript)