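; BP_SwitchName is a railway actor that displays a switch's name on two widget panels.
; On BeginPlay it copies SwitchName into both W_SwitchName widgets, then starts a looping timer.
; The timer culls the panels by camera distance against PanelCullDistance, despite its viewport-themed event name, toggling visibility only on state changes.
; Without a valid camera manager, the panels are shown.
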(event Custom|IsOnViewPort?
  (bind _returnvalue (Game|GetPlayerCameraManager 0))
  ;[1 1 1] On a delay we check if the panel is on screen, if it is not then set hidden in game
  (Utilities|IsValid _returnvalue
    (:Is%20Valid
      (if (< (Math|Vector|VectorLength (- (Transformation|GetActorLocation _returnvalue) (Transformation|GetActorLocation self))) (Variables|Default|GetPanelCullDistance))
        (if (Variables|Default|GetHidden) :!label _label
          (Variables|Default|SetHidden false)
          (Development|SetHiddeninGame (Variables|Default|GetWidget) false false))
        (elif (not (Variables|Default|GetHidden))
          (Variables|Default|SetHidden true)
          (Development|SetHiddeninGame (Variables|Default|GetWidget) true false))))
    (:Is%20Not%20Valid
      (goto _label))))

(event EventBeginPlay
  (bind _asw_switch_name (Utilities|Casting|CastToW_SwitchName (UserInterface|GetUserWidgetObject (Variables|Default|GetWidget1))))
  (Variables|/Game/UI/TrainTemplate/W_SwitchName.W_SwitchName_C|SetName _asw_switch_name (Variables|Default|GetSwitchName))
  (bind _asw_switch_name_2 (Utilities|Casting|CastToW_SwitchName (UserInterface|GetUserWidgetObject (Variables|Default|GetWidget))))
  (Variables|/Game/UI/TrainTemplate/W_SwitchName.W_SwitchName_C|SetName _asw_switch_name_2 (Variables|Default|GetSwitchName))
  ;[1 1 1] On a delay we check if the panel is on screen, if it is not then set hidden in game
  (Utilities|Time|SetTimerbyEvent (delegate Custom|IsOnViewPort?) 3.0 true))

(fn ConstructionScript)