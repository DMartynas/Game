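; BP_BrakeLever is a VR lever interactible that controls the brake on the locomotive.
; Each tick it normalizes the VR lever angle across its negative and positive limits to a 0–1 value and sends it to BP_LocomotiveVR through SetBrakeMessage.
; Gripping the lever enables ticking, which switches off once the lever is neither held nor lerping.
; The construction script finds the locomotive reference with GetActorOfClass.
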(event EventBeginPlay)

(event Collision|EventActorBeginOverlap
  (params (OtherActor :type Actor%20Object%20Reference)))

(event EventTick
  (params (DeltaSeconds :type Float%20%28single-precision%29))
  (CallFunction|UpdateAngle) ; Sets text
  (bind _bcurisheld (Class|VRLeverComponent|IsHeld (Variables|Default|GetVRLever)))
  (if (not _bcurisheld)
    (if (not (Variables|/Script/VRExpansionPlugin.VRLeverComponent|GetbIsLerping (Variables|Default|GetVRLever)))
      (Actor|Tick|SetActorTickEnabled false))))

(event EventOnChildGrip
  (params (GrippingController :type Grip%20Motion%20Controller%20Component%20Object%20Reference) (GripInformation :type BP%20Actor%20Grip%20Information%20Structure%20%28by%20ref%29))
  (Actor|Tick|SetActorTickEnabled true))

(event EventOnChildGripRelease
  (params (ReleasingController :type Grip%20Motion%20Controller%20Component%20Object%20Reference) (GripInformation :type BP%20Actor%20Grip%20Information%20Structure%20%28by%20ref%29) (bWasSocketed :type Boolean)))

(fn ConstructionScript
  (bind _returnvalue (Actor|GetActorOfClass "/Game/Blueprints/Train/Carriage/BP_Carriage_Master/Blueprints/BP_LocomotiveVR.BP_LocomotiveVR_C"))
  (Variables|Default|SetTrainRef _returnvalue))

(fn UpdateAngle
  (bind _vrlever (Variables|Default|GetVRLever))
  (bind _leverlimitnegative (Variables|/Script/VRExpansionPlugin.VRLeverComponent|GetLeverLimitNegative _vrlever))
  (bind _returnvalue (Math|Float|Absolute(Float) _leverlimitnegative))
  (bind _output_get (Variables|Default|SetoutValue (/ (+ (Variables|/Script/VRExpansionPlugin.VRLeverComponent|GetCurrentLeverAngle _vrlever) _returnvalue) (+ _returnvalue (Variables|/Script/VRExpansionPlugin.VRLeverComponent|GetLeverLimitPositive _vrlever)))))
  (Class|TrainInterface|SetBrake(Message) (Variables|Default|GetTrainRef) _output_get))