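; BP_RotarySwitch is a grip-operated rotary switch on the train, attached to the train body's RotarySwitch socket at construction and given a fixed relative location on BeginPlay.
; While gripped, a gated 0.01-second delay loop passes the interacting sphere's physics angular velocity to RecordRotation and applies the result as local roll.
; On release, it applies the roll from RotateToClosestPosition to snap the switch and closes the gate.
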(event Custom|StartInteracting%28GripButton%29_1
  (params (Sphere :type Static%20Mesh%20Component%20Object%20Reference))
  (Utilities|FlowControl|Sequence
    (:then_0
      (goto _label Open))
    (:then_1
      (Utilities|FlowControl|Gate true :!label _label
        (:Exit
          (Utilities|FlowControl|Sequence
            (:then_0
              (bind _returnvalue (Class|RotarySwitch|RecordRotation (Physics|GetPhysicsAngularVelocityinDegrees Sphere "None")))
              (Transformation|AddActorLocalRotation (Math|Rotator|MakeRotator _returnvalue 0.0 0.0) false true))
            (:then_1
              (Utilities|FlowControl|RetriggerableDelay 0.01)
              (goto _label))))))))

(event Custom|StopInteracting%28GripButton%29_1
  (bind _returnvalue (Class|RotarySwitch|RotatetoClosestPosition))
  (Transformation|AddActorLocalRotation (Math|Rotator|MakeRotator _returnvalue 0.0 0.0) false true)
  (Utilities|FlowControl|Gate true) ; enters at Close
)

(event EventBeginPlay
  (Transformation|SetActorRelativeLocation "149.360306,-12.237911,137.950623"))

(event Collision|EventActorBeginOverlap
  (params (OtherActor :type Actor%20Object%20Reference)))

(event EventTick
  (params (DeltaSeconds :type Float%20%28single-precision%29)))

(fn ConstructionScript
  (Transformation|AttachComponentToComponent (Variables|Default|GetTrainBody (.TrainRef (Variables|Default|GetTrainRef))) "RotarySwitch" "KeepRelative" "KeepWorld" "KeepWorld" false))