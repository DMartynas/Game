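; VR reverser control that sets the gear on the BP_LocomotiveVR found at construction.
; While gripped, Tick converts the dial angle to a gear in 45-degree steps; release disables Tick and sends the rounded gear, or zero if the signed offset fails a tolerance check.
; A looping timer polls the train's forward and backward states to block dial travel toward the opposite direction.
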(event Custom|AllowReverserAngles
  (bind _trainref (Variables|Default|GettrainRef))
  (bind _bgoingbackward (Default|GetBackward _trainref))
  (CallFunction|SetNoForward _bgoingbackward)
  (bind _bgoingforward (Default|GetForward _trainref))
  (CallFunction|SetNoBackward _bgoingforward))

(event EventBeginPlay
  (Utilities|Time|SetTimerbyEvent (delegate Custom|AllowReverserAngles) 0.1 true))

(event EventTick
  (params (DeltaSeconds :type Float%20%28single-precision%29))
  (Variables|Default|SetcurrentGear (/ (Variables|/Script/VRExpansionPlugin.VRDialComponent|GetCurrentDialAngle (Variables|Default|GetVRDial)) 45.0)))

(event EventOnChildGrip
  (params (GrippingController :type Grip%20Motion%20Controller%20Component%20Object%20Reference) (GripInformation :type BP%20Actor%20Grip%20Information%20Structure%20%28by%20ref%29))
  (Actor|Tick|SetActorTickEnabled true) ; The dial components tick is off
)

(event EventOnChildGripRelease
  (params (ReleasingController :type Grip%20Motion%20Controller%20Component%20Object%20Reference) (GripInformation :type BP%20Actor%20Grip%20Information%20Structure%20%28by%20ref%29) (bWasSocketed :type Boolean))
  (bind _currentgear (Variables|Default|GetcurrentGear))
  (bind _trainref (Variables|Default|GettrainRef))
  (bind _returnvalue (Math|Float|Round _currentgear))
  (if (< (- _currentgear (Math|Conversions|ToFloat(Integer) _returnvalue)) 1e-06)
    (Class|TrainInterface|SetGear(Message) _trainref _returnvalue)
    (else
      (Class|TrainInterface|SetGear(Message) _trainref)))
  (Actor|Tick|SetActorTickEnabled false))

(fn ConstructionScript
  (bind _returnvalue (Actor|GetActorOfClass "/Game/Blueprints/Train/Carriage/BP_Carriage_Master/Blueprints/BP_LocomotiveVR.BP_LocomotiveVR_C"))
  (Variables|Default|SettrainRef _returnvalue))

(fn SetNoBackward
  (params (bGoingForward :type Boolean))
  (bind _vrdial (Variables|Default|GetVRDial))
  (if bGoingForward
    (Variables|/Script/VRExpansionPlugin.VRDialComponent|SetCClockwiseMaximumDialAngle _vrdial 0.0)
    (else
      (Variables|/Script/VRExpansionPlugin.VRDialComponent|SetCClockwiseMaximumDialAngle _vrdial 45.0))))

(fn SetNoForward
  (params (bGoingBackward :type Boolean))
  (bind _vrdial (Variables|Default|GetVRDial))
  (if bGoingBackward
    (Variables|/Script/VRExpansionPlugin.VRDialComponent|SetClockwiseMaximumDialAngle _vrdial 0.0)
    (else
      (Variables|/Script/VRExpansionPlugin.VRDialComponent|SetClockwiseMaximumDialAngle _vrdial 45.0))))

(fn GetBackward
  (return false))

(fn GetBrakingPressure
  (return 0.0))

(fn GetDiesel
  (return 0.0))

(fn GetForward
  (return false))

(fn GetIncline
  (return 0.0))

(fn GetPressureReserve
  (return 0.0))

(fn GetSand
  (return 0.0))

(fn GetSpeed
  (return 0.0))