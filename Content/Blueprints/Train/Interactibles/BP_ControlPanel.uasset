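; Train control panel actor that builds its driving controls, gauges and buttons at runtime on named sockets of the Panel mesh.
; On BeginPlay, SpawnAndAttachLever spawns and attaches each instrument, shared-class buttons mostly differentiated by ButtonFunction, plus a holo slot and test part.
; BeginPlay then snaps each control to its socket transform, overriding several mismatched attach sockets and scaling up the brake lever.
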(event EventBeginPlay
  (bind _panel (Variables|Default|GetPanel))
  (bind _returnvalue (Transformation|GetSocketTransform _panel "Brake" "RTS_World"))
  (bind (_location _rotation) (Math|Transform|BreakTransform _returnvalue))
  (CallFunction|SpawnandAttachLever)
  (Utilities|FlowControl|Sequence
    (:then_0
      (Transformation|SetActorTransform (Variables|Default|GetAcceleratorSlider) (Transformation|GetSocketTransform (Variables|Default|GetPanel) "Accelerator" "RTS_World")))
    (:then_1
      (Transformation|SetActorTransform (Variables|Default|GetGearDial) (Transformation|GetSocketTransform (Variables|Default|GetPanel) "Reverser" "RTS_World")))
    (:then_2
      (Transformation|SetActorTransform (Variables|Default|GetBrakeLever) (Math|Transform|MakeTransform _location _rotation "40.000000,40.000000,40.000000")))
    (:then_3
      (Transformation|SetActorTransform (Variables|Default|GetSpeedometer) (Transformation|GetSocketTransform (Variables|Default|GetPanel) "Speedometer" "RTS_World")))
    (:then_4
      (Transformation|SetActorTransform (Variables|Default|GetInclinometer) (Transformation|GetSocketTransform (Variables|Default|GetPanel) "Inclinometer" "RTS_World")))
    (:then_5
      (Transformation|SetActorTransform (Variables|Default|GetlWheelSpin) (Transformation|GetSocketTransform (Variables|Default|GetPanel) "WheelSpinLight" "RTS_World")))
    (:then_6
      (Transformation|SetActorTransform (Variables|Default|GetBrakingPressure) (Transformation|GetSocketTransform (Variables|Default|GetPanel) "BrakingPressure" "RTS_World")))
    (:then_7
      (Transformation|SetActorTransform (Variables|Default|GetPressureReserve) (Transformation|GetSocketTransform (Variables|Default|GetPanel) "PressureReserve" "RTS_World")))
    (:then_8
      (Transformation|SetActorTransform (Variables|Default|GetRailSwitches) (Transformation|GetSocketTransform (Variables|Default|GetPanel) "RailSwitches" "RTS_World")))
    (:then_9
      (Transformation|SetActorTransform (Variables|Default|GetHorn) (Transformation|GetSocketTransform (Variables|Default|GetPanel) "Horn" "RTS_World")))
    (:then_10
      (Transformation|SetActorTransform (Variables|Default|GetEngineSwitch) (Transformation|GetSocketTransform (Variables|Default|GetPanel) "EngineSwitch" "RTS_World")))
    (:then_11
      (Transformation|SetActorTransform (Variables|Default|GetInsideLights) (Transformation|GetSocketTransform (Variables|Default|GetPanel) "InsideLight" "RTS_World")))
    (:then_12
      (Transformation|SetActorTransform (Variables|Default|GetOutsideLights) (Transformation|GetSocketTransform (Variables|Default|GetPanel) "OutsideLight" "RTS_World")))
    (:then_13
      (Transformation|SetActorTransform (Variables|Default|GetSand) (Transformation|GetSocketTransform (Variables|Default|GetPanel) "Sand" "RTS_World")))
    (:then_14
      (Transformation|SetActorTransform (Variables|Default|GetPreviousCar) (Transformation|GetSocketTransform (Variables|Default|GetPanel) "PreviousCar" "RTS_World")))
    (:then_15
      (Transformation|SetActorTransform (Variables|Default|GetNextCar) (Transformation|GetSocketTransform (Variables|Default|GetPanel) "NextCar" "RTS_World")))
    (:then_16
      (Transformation|SetActorTransform (Variables|Default|GetDetachCar) (Transformation|GetSocketTransform (Variables|Default|GetPanel) "DetachCar" "RTS_World")))))

(event EventTick
  (params (DeltaSeconds :type Float%20%28single-precision%29)))

(fn ConstructionScript)

(fn SpawnandAttachLever
  (bind _returnvalue (Game|SpawnActorfromClass "/Game/Plugins/VRAssembling/Blueprints/BP_Slot_Holo.BP_Slot_Holo_C" (Math|Transform|MakeTransform "0, 0, 0") "Undefined" 0 0))
  (Transformation|AttachComponentToComponent _returnvalue (Variables|Default|GetScrewable) "None" "KeepRelative" "KeepRelative" "KeepRelative" true)
  (bind _returnvalue_2 (Game|SpawnActorfromClass "/Game/Plugins/VRAssembling/Blueprints/TESTING/BP_TEST_Part_Mesh.BP_TEST_Part_Mesh_C" (Math|Transform|MakeTransform "0, 0, 0") "Undefined" 0 0))
  (Transformation|AttachComponentToComponent _returnvalue_2 (Variables|Default|GetScrew) "None" "KeepRelative" "KeepRelative" "KeepRelative" true)
  (Utilities|FlowControl|Sequence
    (:then_0
      (bind _returnvalue_3 (Game|SpawnActorfromClass "/Game/Blueprints/VR/VRInteractibles/Lever/NativeLeverActor.NativeLeverActor_C" (Transformation|GetSocketTransform (Variables|Default|GetPanel) "Accelerator" "RTS_World") "AlwaysSpawn" 0 0))
      (bind _output_get (Variables|Default|SetAcceleratorSlider _returnvalue_3))
      (Transformation|AttachComponentToComponent (Variables|/Script/Engine.Actor|GetRootComponent _output_get) (Variables|Default|GetPanel) "Accelerator" "KeepRelative" "SnapToTarget" "KeepWorld" true))
    (:then_1
      (bind _returnvalue_4 (Game|SpawnActorfromClass "/Game/Blueprints/Train/Interactibles/BP_Reverser.BP_Reverser_C" (Transformation|GetSocketTransform (Variables|Default|GetPanel) "Reverser" "RTS_World") "AlwaysSpawn" 0 0))
      (bind _output_get_2 (Variables|Default|SetGearDial _returnvalue_4))
      (Transformation|AttachComponentToComponent (Variables|/Script/Engine.Actor|GetRootComponent _output_get_2) (Variables|Default|GetPanel) "Gear" "KeepRelative" "SnapToTarget" "KeepWorld" true))
    (:then_2
      (bind _returnvalue_5 (Game|SpawnActorfromClass "/Game/Blueprints/Train/Interactibles/BP_BrakeLever.BP_BrakeLever_C" (Transformation|GetSocketTransform (Variables|Default|GetPanel) "Brake" "RTS_World") "AlwaysSpawn" 0 0))
      (bind _output_get_3 (Variables|Default|SetBrakeLever _returnvalue_5))
      (Transformation|AttachComponentToComponent (Variables|/Script/Engine.Actor|GetRootComponent _output_get_3) (Variables|Default|GetPanel) "Gear" "KeepRelative" "SnapToTarget" "KeepWorld" true))
    (:then_3
      (bind _returnvalue_6 (Game|SpawnActorfromClass "/Game/Blueprints/Train/Visuals/BP_Speedometer.BP_Speedometer_C" (Transformation|GetSocketTransform (Variables|Default|GetPanel) "Speedometer" "RTS_World") "AlwaysSpawn" 0 0))
      (bind _output_get_4 (Variables|Default|SetSpeedometer _returnvalue_6))
      (Transformation|AttachComponentToComponent (Variables|/Script/Engine.Actor|GetRootComponent _output_get_4) (Variables|Default|GetPanel) "Speedometer" "KeepRelative" "SnapToTarget" "KeepWorld" true))
    (:then_4
      (bind _returnvalue_7 (Game|SpawnActorfromClass "/Game/Blueprints/Train/Visuals/BP_Inclinometer.BP_Inclinometer_C" (Transformation|GetSocketTransform (Variables|Default|GetPanel) "Inclinometer" "RTS_World") "AlwaysSpawn" 0 0))
      (bind _output_get_5 (Variables|Default|SetInclinometer _returnvalue_7))
      (Transformation|AttachComponentToComponent (Variables|/Script/Engine.Actor|GetRootComponent _output_get_5) (Variables|Default|GetPanel) "Inclinometer" "KeepRelative" "SnapToTarget" "KeepWorld" true))
    (:then_5
      (bind _returnvalue_8 (Game|SpawnActorfromClass "/Game/Blueprints/Train/Visuals/BP_Light.BP_Light_C" (Transformation|GetSocketTransform (Variables|Default|GetPanel) "WheelSpinLight" "RTS_World") "AlwaysSpawn" 0 0))
      (bind _output_get_6 (Variables|Default|SetlWheelSpin _returnvalue_8))
      (Transformation|AttachComponentToComponent (Variables|/Script/Engine.Actor|GetRootComponent _output_get_6) (Variables|Default|GetPanel) "WheelSpinLight" "KeepRelative" "SnapToTarget" "KeepWorld" true))
    (:then_6
      (bind _returnvalue_9 (Game|SpawnActorfromClass "/Game/Blueprints/Train/Visuals/BP_Brakes.BP_Brakes_C" (Transformation|GetSocketTransform (Variables|Default|GetPanel) "BrakingPressure" "RTS_World") "AlwaysSpawn" 0 0))
      (bind _output_get_7 (Variables|Default|SetBrakingPressure _returnvalue_9))
      (Transformation|AttachComponentToComponent (Variables|/Script/Engine.Actor|GetRootComponent _output_get_7) (Variables|Default|GetPanel) "WheelSpin" "KeepRelative" "SnapToTarget" "KeepWorld" true))
    (:then_7
      (bind _returnvalue_10 (Game|SpawnActorfromClass "/Game/Blueprints/Train/Visuals/BP_PressureReserve.BP_PressureReserve_C" (Transformation|GetSocketTransform (Variables|Default|GetPanel) "PressureReserve" "RTS_World") "AlwaysSpawn" 0 0))
      (bind _output_get_8 (Variables|Default|SetPressureReserve _returnvalue_10))
      (Transformation|AttachComponentToComponent (Variables|/Script/Engine.Actor|GetRootComponent _output_get_8) (Variables|Default|GetPanel) "PressureReserve" "KeepRelative" "SnapToTarget" "KeepWorld" true))
    (:then_8
      (bind _returnvalue_11 (Game|SpawnActorfromClass "/Game/Blueprints/Train/Interactibles/BP_Switches.BP_Switches_C" (Transformation|GetSocketTransform (Variables|Default|GetPanel) "RailSwitches" "RTS_World") "AlwaysSpawn" 0 0))
      (bind _output_get_9 (Variables|Default|SetRailSwitches _returnvalue_11))
      (Transformation|AttachComponentToComponent (Variables|/Script/Engine.Actor|GetRootComponent _output_get_9) (Variables|Default|GetPanel) "RailSwitches" "KeepRelative" "SnapToTarget" "KeepWorld" true))
    (:then_9
      (bind _returnvalue_12 (Game|SpawnActorfromClass "/Game/Blueprints/VR/VRInteractibles/Button/BP_TrainButton.BP_TrainButton_C" (Transformation|GetSocketTransform (Variables|Default|GetPanel) "Horn" "RTS_World") "AlwaysSpawn" 0 "NewEnumerator0" 0 0))
      (bind _output_get_10 (Variables|Default|SetHorn _returnvalue_12))
      (Transformation|AttachComponentToComponent (Variables|/Script/Engine.Actor|GetRootComponent _output_get_10) (Variables|Default|GetPanel) "RailSwitches" "KeepRelative" "SnapToTarget" "KeepWorld" true))
    (:then_10
      (bind _returnvalue_13 (Game|SpawnActorfromClass "/Game/Blueprints/VR/VRInteractibles/Button/BP_TrainButton.BP_TrainButton_C" (Transformation|GetSocketTransform (Variables|Default|GetPanel) "OutsideLight" "RTS_World") "AlwaysSpawn" 0 "NewEnumerator3" 0 0))
      (bind _output_get_11 (Variables|Default|SetOutsideLights _returnvalue_13))
      (Transformation|AttachComponentToComponent (Variables|/Script/Engine.Actor|GetRootComponent _output_get_11) (Variables|Default|GetPanel) "RailSwitches" "KeepRelative" "SnapToTarget" "KeepWorld" true))
    (:then_11
      (bind _returnvalue_14 (Game|SpawnActorfromClass "/Game/Blueprints/VR/VRInteractibles/Button/BP_TrainButton.BP_TrainButton_C" (Transformation|GetSocketTransform (Variables|Default|GetPanel) "EngineSwitch" "RTS_World") "AlwaysSpawn" 0 "NewEnumerator2" 0 0))
      (bind _output_get_12 (Variables|Default|SetEngineSwitch _returnvalue_14))
      (Transformation|AttachComponentToComponent (Variables|/Script/Engine.Actor|GetRootComponent _output_get_12) (Variables|Default|GetPanel) "RailSwitches" "KeepRelative" "SnapToTarget" "KeepWorld" true))
    (:then_12
      (bind _returnvalue_15 (Game|SpawnActorfromClass "/Game/Blueprints/VR/VRInteractibles/Button/BP_TrainButton.BP_TrainButton_C" (Transformation|GetSocketTransform (Variables|Default|GetPanel) "InsideLight" "RTS_World") "AlwaysSpawn" 0 "NewEnumerator4" 0 0))
      (bind _output_get_13 (Variables|Default|SetInsideLights _returnvalue_15))
      (Transformation|AttachComponentToComponent (Variables|/Script/Engine.Actor|GetRootComponent _output_get_13) (Variables|Default|GetPanel) "RailSwitches" "KeepRelative" "SnapToTarget" "KeepWorld" true))
    (:then_13
      (bind _returnvalue_16 (Game|SpawnActorfromClass "/Game/Blueprints/VR/VRInteractibles/Button/BP_TrainButton.BP_TrainButton_C" (Transformation|GetSocketTransform (Variables|Default|GetPanel) "Sand" "RTS_World") "AlwaysSpawn" 0 "NewEnumerator1" 0 0))
      (bind _output_get_14 (Variables|Default|SetSand _returnvalue_16))
      (Transformation|AttachComponentToComponent (Variables|/Script/Engine.Actor|GetRootComponent _output_get_14) (Variables|Default|GetPanel) "Sand" "KeepRelative" "SnapToTarget" "KeepWorld" true))
    (:then_14
      (bind _returnvalue_17 (Game|SpawnActorfromClass "/Game/Blueprints/VR/VRInteractibles/Button/BP_TrainButton.BP_TrainButton_C" (Transformation|GetSocketTransform (Variables|Default|GetPanel) "PreviousCar" "RTS_World") "AlwaysSpawn" 0 "NewEnumerator6" 0 0))
      (bind _output_get_15 (Variables|Default|SetPreviousCar _returnvalue_17))
      (Transformation|AttachComponentToComponent (Variables|/Script/Engine.Actor|GetRootComponent _output_get_15) (Variables|Default|GetPanel) "PreviousCar" "KeepRelative" "SnapToTarget" "KeepWorld" true))
    (:then_15
      (bind _returnvalue_18 (Game|SpawnActorfromClass "/Game/Blueprints/VR/VRInteractibles/Button/BP_TrainButton.BP_TrainButton_C" (Transformation|GetSocketTransform (Variables|Default|GetPanel) "NextCar" "RTS_World") "AlwaysSpawn" 0 "NewEnumerator5" 0 0))
      (bind _output_get_16 (Variables|Default|SetNextCar _returnvalue_18))
      (Transformation|AttachComponentToComponent (Variables|/Script/Engine.Actor|GetRootComponent _output_get_16) (Variables|Default|GetPanel) "NextCar" "KeepRelative" "SnapToTarget" "KeepWorld" true))
    (:then_16
      (bind _returnvalue_19 (Game|SpawnActorfromClass "/Game/Blueprints/VR/VRInteractibles/Button/BP_TrainButton.BP_TrainButton_C" (Transformation|GetSocketTransform (Variables|Default|GetPanel) "DetachCar" "RTS_World") "AlwaysSpawn" 0 "NewEnumerator7" 0 0))
      (bind _output_get_17 (Variables|Default|SetDetachCar _returnvalue_19))
      (Transformation|AttachComponentToComponent (Variables|/Script/Engine.Actor|GetRootComponent _output_get_17) (Variables|Default|GetPanel) "DetachCar" "KeepRelative" "SnapToTarget" "KeepWorld" true))))

(fn Test)